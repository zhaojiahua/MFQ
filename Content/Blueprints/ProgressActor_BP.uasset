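; ProgressActor_BP is an actor that displays progress, apparently the time remaining on a task, as a scaled, colored mesh.
; Its Construction Script sets the main mesh's relative Y scale to task life minus passed age, leaving X and Z at 1.
; It also creates a dynamic material instance on the sub-mesh and applies the progress color through a vector parameter.
; The event graph has no active logic.
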(fn `UserConstructionScript`
  (`SceneComponent.SetRelativeScale3D` (`self.meshComp`) (`KismetMathLibrary.MakeVector` 1.0 (`KismetMathLibrary.Conv_IntToDouble` (- (`self.mTaskLife`) (`self.mPassAge`))) 1.0))
  (bind _returnvalue (`PrimitiveComponent.CreateDynamicMaterialInstance` (`self.subMeshComp`) 0 "/Game/Meshes/Mats/ProgressMat.ProgressMat" "None"))
  (`MaterialInstanceDynamic.SetVectorParameterValue` _returnvalue "ProgressMatColor" (`KismetMathLibrary.Conv_ColorToLinearColor` (`self.proColor`))))